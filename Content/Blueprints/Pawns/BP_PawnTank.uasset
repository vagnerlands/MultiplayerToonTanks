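; Tank pawn Blueprint that gives a possessing player an on-screen health bar.
; On possession, it checks the controller's pawn, casts to PlayerController, then creates a BP_HealthBar widget, stores it, adds it to that player's screen and initializes it to full.
; The UpdateHealthBar event forwards current and maximum health to the stored widget.
; A debug print of the widget's name remains in the setup.
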(event EventBeginPlay)

(event EventUpdateHealthBar
  (params (CurrentHealth :type Float%20%28single-precision%29) (MaxHealth :type Float%20%28single-precision%29))
  (Default|UpdateHealthBar (Variables|Default|GetHealthBarRef) CurrentHealth MaxHealth))

(event EventPossessed
  (params (NewController :type Controller%20Object%20Reference))
  (Utilities|IsValid (Pawn|GetControlledPawn NewController)
    (:Is%20Valid
      (bind _asplayer_controller (Utilities|Casting|CastToPlayerController (Pawn|GetController)))
      (bind _returnvalue (UserInterface|CreateWidget "/Game/Blueprints/Widgets/BP_HealthBar.BP_HealthBar_C" _asplayer_controller))
      ;[1 1 1] debug
      (Development|PrintString (Utilities|GetDisplayName _returnvalue))
      (bind _output_get (Variables|Default|SetHealthBarRef _returnvalue))
      (UserInterface|Viewport|AddtoPlayerScreen _output_get)
      (Default|UpdateHealthBar _output_get 1.0 1.0))))

(fn ConstructionScript)